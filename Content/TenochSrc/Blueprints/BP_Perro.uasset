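; BP_Perro is a companion actor that hovers ahead of the player and drifts toward nearby points of interest.
; Each Tick it targets a spot in front of the player pawn, or the first POI near that spot, and eases there with VInterpTo.
; It turns opposite to the player's forward direction, without sweeping for collisions as it moves.
; A ShowDialog event makes its widget visible for a few seconds, then hides it.
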(event `ShowDialog`
  (`SceneComponent.SetVisibility` (`self.Widget`) true false)
  (`KismetSystemLibrary.Delay` 5.0)
  (`SceneComponent.SetVisibility` (`self.Widget`) false false))

(event `self.ReceiveTick`
  (params (DeltaSeconds :type "Float (single-precision)"))
  (bind _returnvalue (`GameplayStatics.GetPlayerPawn` 0))
  (bind _output_get (set `self.PlayerLocation` (+ (`self.K2_GetActorLocation` _returnvalue) (* (`self.GetActorForwardVector` _returnvalue) 300))))
  (set `self.GoToSpot` _output_get)
  (for _array_element (`self.POIs`)
    (bind _returnvalue_2 (`self.K2_GetActorLocation` _array_element))
    (if (<= (`KismetMathLibrary.Vector_Distance` _returnvalue_2 (`self.PlayerLocation`)) 450.0)
      (set `self.GoToSpot` _returnvalue_2)
      (break)))
  (`self.K2_SetActorLocation` (`KismetMathLibrary.VInterpTo` (`self.K2_GetActorLocation`) (`self.GoToSpot`) DeltaSeconds 1.0))
  (`self.K2_SetActorRotation` (`KismetMathLibrary.Conv_VectorToRotator` (`KismetMathLibrary.GreaterGreater_VectorRotator` (-1.0 0.0 0.0) (`self.K2_GetActorRotation` (`GameplayStatics.GetPlayerPawn` 0))))))

(fn `NewFunction_0`)

(fn `UserConstructionScript`)